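; Zombie AI character that wanders, chases the player on sight, and drains player health during a button-mash event.
; PawnSensing stores the player and starts a chase, with a retriggerable delay clearing sight memory.
; Tick runs only once a player is stored, either looping delayed damage with rising camera post-process weight or moving to random reachable points when unaware.
; A DisableAIMovement flag gates movement.
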(event OnSeePawn(PawnSensing)
  (params (Pawn :type Pawn%20Object%20Reference))
  (bind _asbp_player_movement (Utilities|Casting|CastToBP_PlayerMovement Pawn))
  (Variables|Default|SetPlayerActor _asbp_player_movement)
  (if (Variables|Default|GetDisableAIMovement)
    (Components|Movement|StopMovementImmediately (Variables|Character|GetCharacterMovement))
    (else
      (bind _asbp_player_movement_2 (Utilities|Casting|CastToBP_PlayerMovement _asbp_player_movement))
      (if (not (Variables|Default|GetDisableAIMovement))
        (Utilities|FlowControl|Sequence
          (:then_0
            ;[1 1 1] Chase Player As Soon As AI Sees Player
            (if (not (Variables|Default|GetDisableAIMovement))
              (Variables|Default|SetCanSeePlayer true)
              (AI|AIMoveTo self "0, 0, 0" _asbp_player_movement_2 5.0 false
                (:then
                  (Variables|Default|SetIsMoving true))
                (:OnSuccess
                  (Variables|Default|SetIsMoving false)))))
          (:then_1
            (Utilities|FlowControl|RetriggerableDelay 3.5) ; How long the AI will remember where the player is
            (Variables|Default|SetCanSeePlayer false)))))))

(event EventTick
  (params (DeltaSeconds :type Float%20%28single-precision%29))
  (bind _asbp_player_movement (Utilities|Casting|CastToBP_PlayerMovement (Variables|Default|GetPlayerActor)))
  (if (Variables|/Game/Blueprints/Player/BP_PlayerMovement.BP_PlayerMovement_C|GetButtonMashEvent _asbp_player_movement) :!label _label
    ;[1 1 1] Damage Deal To Player
    (Utilities|FlowControl|Delay 0.2)
    (bind _asbp_player_movement_2 (Utilities|Casting|CastToBP_PlayerMovement (Variables|Default|GetPlayerActor)))
    (Variables|/Game/Blueprints/Player/BP_PlayerMovement.BP_PlayerMovement_C|SetHealth _asbp_player_movement_2 (- (Variables|/Game/Blueprints/Player/BP_PlayerMovement.BP_PlayerMovement_C|GetHealth _asbp_player_movement_2) 1e+01))
    (bind _output_get (Variables|Default|SetCurrentBlendWeight (+ (Variables|Default|GetCurrentBlendWeight) 0.1)))
    (Class|CameraComponent|SetPostProcessBlendWeight (Variables|/Game/Blueprints/Player/BP_PlayerMovement.BP_PlayerMovement_C|GetMainCam _asbp_player_movement_2) _output_get)
    (goto _label)
    (else
      ;[1 1 1] Wait A Random Amount Of Time
      (if (not (Variables|Default|GetCanSeePlayer))
        (if (not (Variables|Default|GetDisableAIMovement))
          (Utilities|FlowControl|Delay (Math|Random|RandomFloatinRange 2.0 4.0))
          ;[1 1 1] Move AI To A Random Location Within A Radius Of 4000 From Itself
          (AI|AIMoveTo self (.RandomLocation (AI|Navigation|GetRandomReachablePointinRadius (Transformation|GetActorLocation) 4e+03 0 0)) 0 5.0 true
            (:then
              (Variables|Default|SetIsMoving true))
            (:OnSuccess
              (Variables|Default|SetIsMoving false))))))))

(fn ConstructionScript)