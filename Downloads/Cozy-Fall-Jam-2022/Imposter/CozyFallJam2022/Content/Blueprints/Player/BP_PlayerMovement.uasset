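; Player Blueprint for a zombie game, handling a slot inventory, item use, zombie grabs, HUD and level reload on death.
; Tagged pickups fill SlotsArray, and the scrolled slot sets the held mesh and can be dropped or used.
; Medkits restore health, while limited-use torches line-trace to briefly stun zombies.
; Zombie hits lock movement until a Space-started, self-repeating counter passes a random threshold, leaving the zombie temporarily frozen.
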(event EventTick
  (params (DeltaSeconds :type Float%20%28single-precision%29))
  ;[1 1 1] Death Mechanic + Button Mash Threshold Check
  (if (<= (Variables|Default|GetHealth) 0.0)
    (bind _returnvalue (Game|GetCurrentLevelName true))
    (Game|OpenLevel(byName) (Utilities|String|StringToName _returnvalue))
    (else
      (Variables|Default|SetExceedTotalMashes (> (Variables|Default|GetCurrentMashesDone) (Variables|Default|GetTotalMashesNeeded))))))

(event EventBeginPlay
  ;[1 1 1] Display HUD
  (bind _returnvalue (UserInterface|CreateWidget "/Game/Crosshair/HUD.HUD_C"))
  (UserInterface|Viewport|AddtoViewport _returnvalue 0))

(event Collision|EventHit
  (params (MyComp :type Primitive%20Component%20Object%20Reference) (Other :type Actor%20Object%20Reference) (OtherComp :type Primitive%20Component%20Object%20Reference) (bSelfMoved :type Boolean) (HitLocation :type Vector :default "0, 0, 0") (HitNormal :type Vector :default "0, 0, 0") (NormalImpulse :type Vector :default "0, 0, 0") (Hit :type Hit%20Result%20Structure%20%28by%20ref%29))
  ;[1 1 1] Button Mash
  (if (not (Variables|Default|GetButtonMashEvent))
    (bind _asbp_zombie_ai (Utilities|Casting|CastToBP_ZombieAI Other))
    (Variables|Default|SetZombie _asbp_zombie_ai)
    (Variables|Default|SetButtonMashEvent true)
    (Variables|Default|SetTotalMashesNeeded (Math|Random|RandomIntegerinRange 5 15))
    (Variables|Default|SetMovementInput false)))

(event Collision|EventActorBeginOverlap
  (params (OtherActor :type Actor%20Object%20Reference))
  ;[1 1 1] Check if player can pickup item
  (if (Actor|ActorHasTag OtherActor "PickUp")
    (Development|PrintString "Can Be Picked Up")
    (Variables|Default|SetPickUp%20Enable true)
    (Variables|Default|SetActorToBePickedUp OtherActor)))

(event Collision|EventActorEndOverlap
  (params (OtherActor :type Actor%20Object%20Reference))
  ;[1 1 1] Check if player can pickup item
  (Variables|Default|SetPickUp%20Enable false)
  (Development|PrintString "Can't Be Picked Up")
  (Variables|Default|SetPickUp%20Enable false))

(event Input|ActionEvents|InputActionUIMenu
  (params (Key :type Key%20Structure :default "None"))
  ;[1 1 1] Show All Your Inventory
  (:Pressed
    (bind _returnvalue (UserInterface|CreateWidget "/Game/InventoryUI/InventoryMenu.InventoryMenu_C"))
    (bind _output_get (Variables|Default|SetInventoryMenu _returnvalue))
    (UserInterface|Viewport|AddtoViewport _output_get 0)))

(event Input|KeyboardEvents|F
  (params (Key :type Key%20Structure :default "None"))
  (bind _slotsarray (Variables|Default|GetSlotsArray))
  (bind _currentslot (Variables|Default|GetCurrentSlot))
  (bind _inhand (Variables|Default|GetInHand))
  (bind _inhand_2 (Variables|Default|GetInHand))
  (bind _output (Utilities|Array|Get(acopy) _slotsarray _currentslot))
  ;[1 1 1] Drop Item
  (:Pressed
    (if (!= _output 0)
      (bind _returnvalue (Game|SpawnActorfromClass (Utilities|GetClass _output) (Math|Transform|MakeTransform (.location (Transformation|GetActorTransform)) "0, 0, 0" "1.000000,1.000000,1.000000") "Undefined" 0 0))
      (Development|PrintString (Utilities|GetDisplayName _returnvalue))
      ;;[1 1 1] Remove item from inventory
      (Utilities|Array|SetArrayElem (Variables|Default|GetSlotsArray) (Variables|Default|GetCurrentSlot) 0)
      ;[1 1 1] Change Mesh In Hand
      (if (Utilities|Array|IsEmpty (Utilities|GetDisplayName (Utilities|Array|Get(acopy) (Variables|Default|GetSlotsArray) (Variables|Default|GetCurrentSlot))))
        (Development|PrintString "Show No Mesh (Empty Slot)")
        (Components|StaticMesh|SetStaticMesh (Variables|Default|GetInHand) 0)
        (elif (Actor|ActorHasTag (Utilities|Array|Get(acopy) (Variables|Default|GetSlotsArray) (Variables|Default|GetCurrentSlot)) "Medkit")
          (Components|StaticMesh|SetStaticMesh _inhand_2 "/Game/Blueprints/Objects/Medkit/MedKit.MedKit")
          (Rendering|Material|SetMaterial _inhand_2 0 "/Game/Blueprints/Objects/Medkit/MedkitMat.MedkitMat")
          (Transformation|SetWorldScale3D _inhand_2 "0.100000,0.100000,0.100000")
          (Transformation|SetRelativeRotation _inhand_2 "0, 0, 0" false false)
          (elif (Actor|ActorHasTag (Utilities|Array|Get(acopy) (Variables|Default|GetSlotsArray) (Variables|Default|GetCurrentSlot)) "Torch")
            (Components|StaticMesh|SetStaticMesh _inhand "/Game/Blueprints/Objects/Torch/TorchModel.TorchModel")
            (Rendering|Material|SetMaterial _inhand 0 "/Game/Blueprints/Objects/Torch/TorchMat.TorchMat")
            (Transformation|SetWorldScale3D _inhand "2.000000,2.000000,2.000000")
            (Transformation|SetRelativeRotation _inhand "180.000000, 0, 0" false false)
            (else
              (Development|PrintString "NO CONDITION MET FOR SETTING MESH"))))))))

(event Input|MouseEvents|MouseWheelDown
  (params (Key :type Key%20Structure :default "None"))
  (bind _inhand (Variables|Default|GetInHand))
  (bind _inhand_2 (Variables|Default|GetInHand))
  ;[1 1 1] Go Through Inventory
  (:Pressed
    (if (not (<= (Variables|Default|GetCurrentSlot) 0))
      (bind _output_get (Variables|Default|SetCurrentSlot (- (Variables|Default|GetCurrentSlot) 1)))
      (if (Utilities|Array|IsEmpty (Utilities|GetDisplayName (Utilities|Array|Get(acopy) (Variables|Default|GetSlotsArray) _output_get)))
        (Development|PrintString "Empty Slot")
        (else
          (Development|PrintString (Utilities|GetDisplayName (Utilities|Array|Get(acopy) (Variables|Default|GetSlotsArray) _output_get)))))
      ;[1 1 1] Change Mesh In Hand
      (if (Utilities|Array|IsEmpty (Utilities|GetDisplayName (Utilities|Array|Get(acopy) (Variables|Default|GetSlotsArray) (Variables|Default|GetCurrentSlot))))
        (Development|PrintString "Show No Mesh (Empty Slot)")
        (Components|StaticMesh|SetStaticMesh (Variables|Default|GetInHand) 0)
        (elif (Actor|ActorHasTag (Utilities|Array|Get(acopy) (Variables|Default|GetSlotsArray) (Variables|Default|GetCurrentSlot)) "Medkit")
          (Components|StaticMesh|SetStaticMesh _inhand_2 "/Game/Blueprints/Objects/Medkit/MedKit.MedKit")
          (Rendering|Material|SetMaterial _inhand_2 0 "/Game/Blueprints/Objects/Medkit/MedkitMat.MedkitMat")
          (Transformation|SetWorldScale3D _inhand_2 "0.100000,0.100000,0.100000")
          (Transformation|SetRelativeRotation _inhand_2 "0, 0, 0" false false)
          (elif (Actor|ActorHasTag (Utilities|Array|Get(acopy) (Variables|Default|GetSlotsArray) (Variables|Default|GetCurrentSlot)) "Torch")
            (Components|StaticMesh|SetStaticMesh _inhand "/Game/Blueprints/Objects/Torch/TorchModel.TorchModel")
            (Rendering|Material|SetMaterial _inhand 0 "/Game/Blueprints/Objects/Torch/TorchMat.TorchMat")
            (Transformation|SetWorldScale3D _inhand "2.000000,2.000000,2.000000")
            (Transformation|SetRelativeRotation _inhand "180.000000, 0, 0" false false)
            (else
              (Development|PrintString "NO CONDITION MET FOR SETTING MESH"))))))))

(event Input|MouseEvents|MouseWheelUp
  (params (Key :type Key%20Structure :default "None"))
  (bind _inhand (Variables|Default|GetInHand))
  (bind _inhand_2 (Variables|Default|GetInHand))
  ;[1 1 1] Go Through Inventory
  (:Pressed
    (if (not (>= (Variables|Default|GetCurrentSlot) (Variables|Default|GetInventoryMaxSlots)))
      (bind _output_get (Variables|Default|SetCurrentSlot (+ (Variables|Default|GetCurrentSlot) 1)))
      (if (Utilities|Array|IsEmpty (Utilities|GetDisplayName (Utilities|Array|Get(acopy) (Variables|Default|GetSlotsArray) _output_get)))
        (Development|PrintString "Empty Slot")
        (else
          (Development|PrintString (Utilities|GetDisplayName (Utilities|Array|Get(acopy) (Variables|Default|GetSlotsArray) _output_get)))))
      ;[1 1 1] Change Mesh In Hand
      (if (Utilities|Array|IsEmpty (Utilities|GetDisplayName (Utilities|Array|Get(acopy) (Variables|Default|GetSlotsArray) (Variables|Default|GetCurrentSlot))))
        (Development|PrintString "Show No Mesh (Empty Slot)")
        (Components|StaticMesh|SetStaticMesh (Variables|Default|GetInHand) 0)
        (elif (Actor|ActorHasTag (Utilities|Array|Get(acopy) (Variables|Default|GetSlotsArray) (Variables|Default|GetCurrentSlot)) "Medkit")
          (Components|StaticMesh|SetStaticMesh _inhand_2 "/Game/Blueprints/Objects/Medkit/MedKit.MedKit")
          (Rendering|Material|SetMaterial _inhand_2 0 "/Game/Blueprints/Objects/Medkit/MedkitMat.MedkitMat")
          (Transformation|SetWorldScale3D _inhand_2 "0.100000,0.100000,0.100000")
          (Transformation|SetRelativeRotation _inhand_2 "0, 0, 0" false false)
          (elif (Actor|ActorHasTag (Utilities|Array|Get(acopy) (Variables|Default|GetSlotsArray) (Variables|Default|GetCurrentSlot)) "Torch")
            (Components|StaticMesh|SetStaticMesh _inhand "/Game/Blueprints/Objects/Torch/TorchModel.TorchModel")
            (Rendering|Material|SetMaterial _inhand 0 "/Game/Blueprints/Objects/Torch/TorchMat.TorchMat")
            (Transformation|SetWorldScale3D _inhand "2.000000,2.000000,2.000000")
            (Transformation|SetRelativeRotation _inhand "180.000000, 0, 0" false false)
            (else
              (Development|PrintString "NO CONDITION MET FOR SETTING MESH"))))))))

(event Input|KeyboardEvents|E
  (params (Key :type Key%20Structure :default "None"))
  (bind _slotsarray (Variables|Default|GetSlotsArray))
  (bind _actortobepickedup (Variables|Default|GetActorToBePickedUp))
  ;[1 1 1] PickUp Mechanic
  (:Pressed
    (if (< (Variables|Default|GetInventoryMaxSlots) 0)
      (Development|PrintString "Max Amount In Inventory")
      (elif (Variables|Default|GetPickUp%20Enable)
        (if (Actor|ActorHasTag _actortobepickedup "PickUp")
          (Development|PrintString (Utilities|GetDisplayName _actortobepickedup))
          ;;[1 1 1] Get Which Item It Is
          (if (Actor|ActorHasTag _actortobepickedup "TestOne")
            (Rendering|SetActorHiddenInGame _actortobepickedup true :!label _label)
            (Collision|SetActorEnableCollision _actortobepickedup false)
            ;[1 1 1] Add Item to Inventory
            (bind (_array_element _array_index) (Utilities|Array|ForEachLoopwithBreak _slotsarray :!label _label_2)
              (:LoopBody
                (if (== _array_element 0)
                  (Utilities|Array|SetArrayElem _slotsarray _array_index (Variables|Default|GetActorToBePickedUp))
                  (goto _label_2 Break))))
            (elif (Actor|ActorHasTag _actortobepickedup "TestTwo")
              (goto _label)
              (elif (Actor|ActorHasTag _actortobepickedup "Torch")
                (goto _label)
                (elif (Actor|ActorHasTag _actortobepickedup "Medkit")
                  (goto _label))))))))))

(event Input|MouseEvents|LeftMouseButton
  (params (Key :type Key%20Structure :default "None"))
  (bind _inhand (Variables|Default|GetInHand))
  (bind _inhand_2 (Variables|Default|GetInHand))
  (bind _maincam (Variables|Default|GetMainCam))
  (bind _currentslot (Variables|Default|GetCurrentSlot))
  (bind _slotsarray (Variables|Default|GetSlotsArray))
  (bind _returnvalue (Components|GetOwner _maincam))
  (bind _output (Utilities|Array|Get(acopy) _slotsarray _currentslot))
  (bind _returnvalue_2 (Transformation|GetActorLocation _returnvalue))
  ;[1 1 1] Using Items From Inventory
  (:Pressed
    (if (Utilities|IsValid (Variables|Default|GetInventoryMenu))
      (if (Variables|/Game/InventoryUI/InventoryMenu.InventoryMenu_C|GetIn%20Inventory (Variables|Default|GetInventoryMenu))
        (Development|PrintString "In Inventory")
        (else
          (Development|PrintString (Utilities|String|ToString(Integer) _currentslot) :!label _label)
          (if (Utilities|Array|IsEmpty (Utilities|GetDisplayName _output))
            (Development|PrintString "Nothing Equipped")
            ;[1 1 1] Change Mesh In Hand
            (if (Utilities|Array|IsEmpty (Utilities|GetDisplayName (Utilities|Array|Get(acopy) (Variables|Default|GetSlotsArray) (Variables|Default|GetCurrentSlot)))) :!label _label_2
              (Development|PrintString "Show No Mesh (Empty Slot)")
              (Components|StaticMesh|SetStaticMesh (Variables|Default|GetInHand) 0)
              (elif (Actor|ActorHasTag (Utilities|Array|Get(acopy) (Variables|Default|GetSlotsArray) (Variables|Default|GetCurrentSlot)) "Medkit")
                (Components|StaticMesh|SetStaticMesh _inhand_2 "/Game/Blueprints/Objects/Medkit/MedKit.MedKit")
                (Rendering|Material|SetMaterial _inhand_2 0 "/Game/Blueprints/Objects/Medkit/MedkitMat.MedkitMat")
                (Transformation|SetWorldScale3D _inhand_2 "0.100000,0.100000,0.100000")
                (Transformation|SetRelativeRotation _inhand_2 "0, 0, 0" false false)
                (elif (Actor|ActorHasTag (Utilities|Array|Get(acopy) (Variables|Default|GetSlotsArray) (Variables|Default|GetCurrentSlot)) "Torch")
                  (Components|StaticMesh|SetStaticMesh _inhand "/Game/Blueprints/Objects/Torch/TorchModel.TorchModel")
                  (Rendering|Material|SetMaterial _inhand 0 "/Game/Blueprints/Objects/Torch/TorchMat.TorchMat")
                  (Transformation|SetWorldScale3D _inhand "2.000000,2.000000,2.000000")
                  (Transformation|SetRelativeRotation _inhand "180.000000, 0, 0" false false)
                  (else
                    (Development|PrintString "NO CONDITION MET FOR SETTING MESH")))))
            (else
              (Development|PrintString "Something Equipped")
              (if (Actor|ActorHasTag _output "TestOne")
                (Development|PrintString "Pickup One")
                (elif (Actor|ActorHasTag _output "TestTwo")
                  (Development|PrintString "Pickup Two")
                  (elif (Actor|ActorHasTag _output "Medkit")
                    (Development|PrintString "Medkit")
                    ;[1 1 1] Medkit Usage
                    (Variables|Default|SetHealth 1e+02)
                    (Class|CameraComponent|SetPostProcessBlendWeight (Variables|Default|GetMainCam) 0.0)
                    ;[1 1 1] Drop Item
                    ;;[1 1 1] Remove item from inventory
                    (Utilities|Array|SetArrayElem (Variables|Default|GetSlotsArray) (Variables|Default|GetCurrentSlot) 0 :!label _label_3)
                    (goto _label_2)
                    (elif (Actor|ActorHasTag _output "Torch")
                      (Development|PrintString "Torch")
                      ;[1 1 1] Torch Usage
                      (if (>= (Variables|Default|GetCurrentTorchUsage) (Variables|Default|GetMaxTorchUsage))
                        (Variables|Default|SetCurrentTorchUsage 0)
                        (goto _label_3)
                        (else
                          (bind _outhit (Collision|LineTraceByChannel (+ _returnvalue_2 "0,0.000000,90.000000") (+ _returnvalue_2 (* (Math|Vector|GetForwardVector (Pawn|GetControlRotation (Pawn|GetController) :!class /Script/Engine.Controller)) (Math|Conversions|ToVector(Float) 5e+03))) "TraceTypeQuery1" false 0 "ForDuration"))
                          (Variables|Default|SetCurrentTorchUsage (+ (Variables|Default|GetCurrentTorchUsage) 1))
                          (bind _asbp_zombie_ai (Utilities|Casting|CastToBP_ZombieAI (.HitActor (Collision|BreakHitResult _outhit))))
                          (Development|PrintString "Hit Zombie With Torch Ray")
                          (bind _output_get (Variables|Default|SetZombie _asbp_zombie_ai))
                          (bind _asbp_zombie_ai_2 (Utilities|Casting|CastToBP_ZombieAI _output_get))
                          (Variables|/Game/Blueprints/AI/BP_ZombieAI.BP_ZombieAI_C|SetIsMoving _asbp_zombie_ai false)
                          (Rendering|SetVisibility (Variables|Default|GetSpotLight) true false)
                          (Variables|/Game/Blueprints/AI/BP_ZombieAI.BP_ZombieAI_C|SetDisableAIMovement _asbp_zombie_ai_2 true)
                          (Variables|/Game/Blueprints/AI/BP_ZombieAI.BP_ZombieAI_C|SetCanSeePlayer _asbp_zombie_ai_2 false)
                          (Utilities|FlowControl|Delay 1.0)
                          (Rendering|SetVisibility (Variables|Default|GetSpotLight) false false)
                          (Utilities|FlowControl|Delay 3.0)
                          (Variables|/Game/Blueprints/AI/BP_ZombieAI.BP_ZombieAI_C|SetDisableAIMovement _asbp_zombie_ai_2 false)))))))))))
      (else
        (goto _label)))))

(event Input|KeyboardEvents|SpaceBar
  (params (Key :type Key%20Structure :default "None"))
  ;[1 1 1] Button Mash
  (:Pressed
    (if (Variables|Default|GetButtonMashEvent) :!label _label
      (bind _asbp_zombie_ai (Utilities|Casting|CastToBP_ZombieAI (Variables|Default|GetZombie)))
      (Variables|/Game/Blueprints/AI/BP_ZombieAI.BP_ZombieAI_C|SetDisableAIMovement _asbp_zombie_ai true)
      (Variables|Default|SetMovementInput false)
      (Variables|Default|SetCurrentMashesDone (+ (Variables|Default|GetCurrentMashesDone) 1))
      (if (Variables|Default|GetExceedTotalMashes)
        (Variables|Default|SetMovementInput true)
        (Variables|Default|SetButtonMashEvent false)
        (Variables|Default|SetCurrentMashesDone 0)
        (Utilities|FlowControl|Delay (Math|Conversions|ToFloat(Integer) (Math|Random|RandomIntegerinRange 5 15)))
        (bind _asbp_zombie_ai_2 (Utilities|Casting|CastToBP_ZombieAI (Variables|Default|GetZombie)))
        (Variables|/Game/Blueprints/AI/BP_ZombieAI.BP_ZombieAI_C|SetDisableAIMovement _asbp_zombie_ai_2 false)
        (else
          (Utilities|FlowControl|Delay 0.1)
          (goto _label))))))

(fn ConstructionScript)

(fn UpdateUI
  (params (NewParam1 :type Slot%20Data%20Structure))
  (bind _slotnumber (Utilities|Struct|BreakSlotData NewParam1))
  (bind _structout (Utilities|Struct|SetmembersinSlotData NewParam1 _slotnumber (Utilities|Text|ToText(String) (Utilities|GetDisplayName (Utilities|Array|Get(acopy) (Variables|Default|GetSlotsArray) _slotnumber)))))
  (return _structout))